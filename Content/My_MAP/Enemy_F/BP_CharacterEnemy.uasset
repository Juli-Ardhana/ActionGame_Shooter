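; Enemy character that patrols, chases the player on sight and shoots with a rifle.
; Patrol loops through random reachable points via AIMoveTo, while PawnSensing sightings start a chase that triggers an attack on arrival.
; Attacks turn the controller toward the target and line-trace from the muzzle along the mesh's right vector, damaging the player on hit.
; Incoming damage drains health and ragdolls the mesh at zero.
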(event OnSeePawn(PawnSensing)
  (params (Pawn :type Pawn%20Object%20Reference))
  ;[1 1 1] When See Player Triggered Chasing
  (Utilities|IsValid Pawn
    (:Is%20Valid
      (Utilities|Casting|CastToBP_ThirdPersonCharacter Pawn)
      (CallFunction|Chasing Pawn))))

(event Custom|Search%20Around%20%28PATROL%29
  ;[1 1 1] Searching Around
  (AI|AIMoveTo self (.RandomLocation (AI|Navigation|GetRandomReachablePointinRadius (Transformation|GetActorLocation) 2e+03 0 0)) 0 4.5e+02 false
    (:OnSuccess
      (Utilities|FlowControl|Delay 0.5)
      (CallFunction|SearchAround(PATROL)))))

(event Custom|Chasing
  (params (TargetActor :type Actor%20Object%20Reference))
  ;[1 1 1] Chasing Player
  (Utilities|IsValid TargetActor
    (:Is%20Valid
      (AI|AIMoveTo self "0, 0, 0" TargetActor 4.5e+02 false
        (:OnSuccess
          (CallFunction|Attacking TargetActor))))))

(event Custom|Attacking
  (params (Target :type Actor%20Object%20Reference))
  (bind _returnvalue (Pawn|GetController))
  (bind _falcon_rifle (Variables|Default|GetFalcon%20Rifle))
  (bind _returnvalue_2 (Transformation|GetSocketTransform _falcon_rifle "Falcon_Muzzle" "RTS_World"))
  ;[1 1 1] Attacking Player
  (Utilities|IsValid _returnvalue
    (:Is%20Valid
      (Pawn|SetControlRotation _returnvalue (Math|Rotator|FindLookatRotation (Transformation|GetActorLocation) (Transformation|GetActorLocation Target)))
      (bind (_outhit _returnvalue_3) (Collision|LineTraceByChannel (.location _returnvalue_2) (+ (.location _returnvalue_2) (* (Math|Vector|GetRightVector (Transformation|GetWorldRotation (Variables|Character|GetMesh))) 2e+03)) "TraceTypeQuery1" false 0 "ForDuration"))
      (if _returnvalue_3
        (bind _asbp_third_person_character (Utilities|Casting|CastToBP_ThirdPersonCharacter (.HitActor (Collision|BreakHitResult _outhit))))
        (Game|Damage|ApplyDamage _asbp_third_person_character 15.0 0 0)))))

(event EventBeginPlay
  (CallFunction|SearchAround(PATROL) self))

(event Game|Damage|EventAnyDamage
  (params (Damage :type Float%20%28single-precision%29) (DamageType :type Damage%20Type%20Object%20Reference) (InstigatedBy :type Controller%20Object%20Reference) (DamageCauser :type Actor%20Object%20Reference))
  ;[1 1 1] Take Any Damage (Enemy)
  (Variables|Default|SetHealth_E (- (Variables|Default|GetHealth_E) Damage))
  (if (<= (Variables|Default|GetHealth_E) 0.0)
    (Physics|SetSimulatePhysics (Variables|Character|GetMesh) true)))

(fn ConstructionScript)