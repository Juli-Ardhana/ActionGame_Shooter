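; BP_SEnemyAI is an enemy character that chases and attacks the player and exposes a patrol route.
; ChasingPlayer moves to the player, triggers the attack montage, then repeats after a delay.
; WieldSword plays a pull-out montage whose notify spawns a sword on the hand socket; dispatchers signal wield and attack completion.
; Helpers handle health reduction, sprint speed changes and checking whether player health is zero.
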(event Custom|Chasing%20Player
  ;[1 1 1] Chasing Player
  (AI|AIMoveTo self "0, 0, 0" (Game|GetPlayerCharacter 0) 1.5e+02 false
    (:OnSuccess
      (CallFunction|Attack)
      (Utilities|FlowControl|Delay 2.0)
      (CallFunction|ChasingPlayer))))

(event Custom|Attack
  ;[1 1 1] Enemy Attack
  (Animation|Montage|PlayMontage (Variables|Character|GetMesh) "/Game/My_MAP/Enemy_F/Smart_enemy_AI/Animation/Attack/AM_Attack.AM_Attack"
    (:OnCompleted
      _)
    (:OnInterrupted
      _))
  (Default|CallOnAttackEnd))

(event Custom|WieldSword
  ;[1 1 1] Weapon Attach to Enemy
  (Variables|Default|SetisWieldingSword false)
  (bind _notifyname (Animation|Montage|PlayMontage 0 "/Game/My_MAP/Enemy_F/Smart_enemy_AI/Animation/Attack/AM_PullOut.AM_PullOut")
    (:OnCompleted
      (Default|CallOnWielding))
    (:OnNotifyBegin
      (switch name _notifyname
        (:Default
          (bind _returnvalue (Game|SpawnActorfromClass "/Game/My_MAP/Enemy_F/Smart_enemy_AI/Weapons/BP_Sword.BP_Sword_C" (Transformation|GetActorTransform) "Undefined" "MultiplyWithRoot" 0 0))
          (Transformation|AttachComponentToComponent _returnvalue (Variables|Character|GetMesh) "Hold_Sword" "SnapToTarget" "SnapToTarget" "SnapToTarget" true))))))

(event EventBeginPlay)

(fn ConstructionScript)

(fn AttackPlayer
  (params (Damage :type Integer))
  (bind _output_get (Variables|Default|SetHealthPoint (- (Variables|Default|GetHealthPoint) Damage)))
  (return _output_get))

(fn PlayerSprint
  (Variables|/Script/Engine.CharacterMovementComponent|SetMaxWalkSpeed (Variables|Character|GetCharacterMovement) (Variables|Default|GetSprintSpeed))
  (Components|Animation|PlayAnimation (Variables|Character|GetMesh) 0 false)
  (if (Variables|Default|GetcanSprint?)
    (Variables|Default|SetcanSprint? true)
    (else
      (Variables|Default|SetcanSprint? false))))

(fn StopSprint
  (Variables|/Script/Engine.CharacterMovementComponent|SetMaxWalkSpeed (Variables|Character|GetCharacterMovement) (Variables|Default|GetWalkMaxSpeed))
  (if (Variables|Default|GetcanSprint?)
    (Variables|Default|SetcanSprint? false)
    (else
      (Variables|Default|SetcanSprint? true))))

(fn GetPatrolRoute
  (return (Variables|Default|GetPatrolRoute)))