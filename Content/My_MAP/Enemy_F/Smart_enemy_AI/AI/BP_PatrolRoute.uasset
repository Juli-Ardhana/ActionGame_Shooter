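; BP_PatrolRoute is a patrol path for enemy AI, built on a spline whose points serve as patrol stops.
; IncrementPatrolRoute advances the point index and flips direction at the last and first points, so movement ping-pongs along the route.
; GetSplinePointasWorldPosition returns the current point's world location for use as a move target.
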(event Custom|Increment%20PatrolRoute
  ;[1 1 1] Patrol Route
  (bind _output_get (Variables|Default|SetPatrolIndex (+ (Variables|Default|GetPatrolIndex) (Variables|Default|GetDIrection))))
  (if (== _output_get (- (Spline|GetNumberOfSplinePoints (Variables|Default|GetPatrol%20Route)) 1))
    (Variables|Default|SetDIrection -1)
    (elif (== (Variables|Default|GetPatrolIndex) 0)
      (Variables|Default|SetDIrection 1))))

(fn ConstructionScript)

(fn GetSplinePointasWorldPosition
  (return (Spline|GetLocationatSplinePoint (Variables|Default|GetPatrol%20Route) (Variables|Default|GetPatrolIndex) "World")))