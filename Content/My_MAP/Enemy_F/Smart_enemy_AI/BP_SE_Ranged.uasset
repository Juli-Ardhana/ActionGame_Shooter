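; BP_SE_Ranged is a rifle-wielding ranged enemy character for the smart enemy AI, with a widget health bar.
; It attaches a spawned rifle to its Weapon socket, then plays a firing montage on attack and signals when it ends.
; A montage notify line-traces from the rifle to the AI controller's target, but the hit applies no damage yet.
; Functions supply movement speed, ideal ranges and patrol route, and forward incoming damage to BPCDamageSystem.
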(event EventBeginPlay
  (CallFunction|EquipWeapon)
  (bind _returnvalue (UserInterface|CreateWidget "/Game/My_MAP/Enemy_F/Smart_enemy_AI/AI/DamageSystem/WB_EnemyHP.WB_EnemyHP_C" 0 self 0))
  (UserInterface|SetWidget (Variables|Default|GetEnemy_HP) _returnvalue))

(event EventEquipWeapon
  ;[1 1 1] Equip Weapon Gun
  (bind _returnvalue (Game|SpawnActorfromClass "/Game/My_MAP/Enemy_F/Smart_enemy_AI/Weapons/BP-WeaponRifle.BP-WeaponRifle_C" (Math|Transform|MakeTransform "0, 0, 0") "Undefined" "MultiplyWithRoot" 0 0))
  (bind _output_get (Variables|Default|SetWeaponActor _returnvalue))
  (Transformation|AttachComponentToComponent _output_get (Variables|Character|GetMesh) "Weapon" "SnapToTarget" "SnapToTarget" "SnapToTarget" true)
  (Variables|Default|SetisWieldingWeapon true)
  (Default|CallOnEquipWeapon))

(event EventAttack
  ;[1 1 1] Attack to Player
  (bind _notifyname (Animation|Montage|PlayMontage (Variables|Character|GetMesh) "/Game/My_MAP/Enemy_F/Smart_enemy_AI/SE_Ranged/Animation/Based_Anim/Rifle_anim/Montage/AM_Firing_rifle.AM_Firing_rifle")
    (:OnCompleted
      (Default|CallOnAttackEnd :!label _label))
    (:OnInterrupted
      (goto _label))
    (:OnNotifyBegin
      (switch name _notifyname
        (:Shooting
          (bind _asaic_enemey_base (Utilities|Casting|CastToAIC_Enemey_Base (AI|GetAIController self)))
          (bind _attack_target (Variables|/Game/My_MAP/Enemy_F/Smart_enemy_AI/AI/AIC_Enemey_Base.AIC_Enemey_Base_C|GetAttack%20Target _asaic_enemey_base)
            (:then
              (bind _returnvalue (Collision|LineTraceByChannel (Transformation|GetActorLocation (Variables|Default|GetWeaponActor)) (Transformation|GetActorLocation _attack_target) "TraceTypeQuery1" false 0 "ForDuration"))
              (if _returnvalue
                _))
            (:else)))))))

(fn ConstructionScript
  (|CallParentFunction))

(fn SetMovementSpeed
  (params (Speed :type E_MovementSpeed%20Enum :default "NewEnumerator0"))
  (bind _output_get (Variables|/Script/Engine.CharacterMovementComponent|SetMaxWalkSpeed (Variables|Character|GetCharacterMovement) (Utilities|Select :Index Speed :NewEnumerator0 0.0 :NewEnumerator1 2e+02 :NewEnumerator2 3e+02 :NewEnumerator3 5e+02)))
  (return _output_get))

(fn GetIdealRange
  (return 6e+02 6e+02))

(fn GetPatrolRoute
  (return (Variables|Default|GetPatrolRoute)))

(fn TakeDamage
  (params (DamageInfo :type S%20Damage%20Info%20Structure))
  (bind _wasdamage (Default|TakeDamage (Variables|Default|GetBPC_DamageSystem) DamageInfo))
  (return _wasdamage))