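; BP_SE_Melee is a melee smart-AI enemy with a health bar widget and fixed attack and defend ranges.
; Attack plays a random AttackCombo montage and signals attack end on completion or interruption.
; Equip and unequip montages use notifies to set the wielding state and call back when finished.
; The equip notify spawns and socket-attaches a sword, while the destroy call for unequipping is disconnected.
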(event EventEquipWeapon
  ;[1 1 1] Weapon Attach to Enemy
  (bind _notifyname (Animation|Montage|PlayMontage (Variables|Character|GetMesh) "/Game/My_MAP/Enemy_F/Smart_enemy_AI/SE_Melee/Attack/Montage/AM_Draw_Melee.AM_Draw_Melee")
    (:OnCompleted
      (Default|CallOnEquipWeapon :!label _label))
    (:OnInterrupted
      (goto _label))
    (:OnNotifyBegin
      (switch name _notifyname
        (:Draw%20Sword
          (bind _returnvalue (Game|SpawnActorfromClass "/Game/My_MAP/Enemy_F/Smart_enemy_AI/Weapons/BP_WeaponSword2.BP_WeaponSword2_C" (Transformation|GetActorTransform) "Undefined" "MultiplyWithRoot" 0 0))
          (bind _output_get (Variables|Default|SetWeaponActor _returnvalue))
          (Transformation|AttachComponentToComponent _output_get (Variables|Character|GetMesh) "Weapon_Melee" "SnapToTarget" "SnapToTarget" "SnapToTarget" true)
          (Variables|Default|SetisWieldingWeapon true))))))

(event EventUnequipWeapon
  ;[1 1 1] Sheathed Enemy
  (bind _notifyname (Animation|Montage|PlayMontage (Variables|Character|GetMesh) "/Game/My_MAP/Enemy_F/Smart_enemy_AI/SE_Melee/Attack/Montage/AM_Sheathed_Melee.AM_Sheathed_Melee")
    (:OnCompleted
      (Default|CallOnUnequipWeapon))
    (:OnNotifyBegin
      (switch name _notifyname
        (:PutAway_Melee
          (Variables|Default|SetisWieldingWeapon false))))))

(event EventAttack
  (bind _attackcombo (Variables|Default|GetAttackCombo))
  ;[1 1 1] Enemy Attack
  (Animation|Montage|PlayMontage (Variables|Character|GetMesh) (Utilities|Array|Get(acopy) _attackcombo (Math|Random|RandomInteger (Utilities|Array|Length _attackcombo)))
    (:OnCompleted
      _)
    (:OnInterrupted
      _))
  (Default|CallOnAttackEnd))

(event EventBeginPlay
  (bind _returnvalue (UserInterface|CreateWidget "/Game/My_MAP/Enemy_F/Smart_enemy_AI/AI/DamageSystem/WB_EnemyHP.WB_EnemyHP_C" 0 self 0))
  (UserInterface|SetWidget (Variables|Default|GetEnemy_HP) _returnvalue))

(fn ConstructionScript
  (|CallParentFunction))

(fn GetIdealRange
  (return 135.0 3e+02))