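; BP_DoorS_3 is an automatic two-part door that opens when a BP_Macky actor enters its trigger Box and closes when it leaves.
; Begin overlap plays the Door3 timeline, which drives the relative locations of Door3 and Door3A from separate tracks.
; End overlap reverses the same timeline, and both events store the BP_Macky reference and play the MSS_DoorOpen sound at the door's location.
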(event OnComponentBeginOverlap(Box)
  (params (OverlappedComponent :type Primitive%20Component%20Object%20Reference) (OtherActor :type Actor%20Object%20Reference) (OtherComp :type Primitive%20Component%20Object%20Reference) (OtherBodyIndex :type Integer) (bFromSweep :type Boolean) (SweepResult :type Hit%20Result%20Structure%20%28by%20ref%29))
  (bind _asbp_macky (Utilities|Casting|CastToBP_Macky OtherActor))
  (Variables|Default|SetBP_Macky _asbp_macky)
  (Audio|PlaySoundatLocation "/Game/My_MAP/MK_Character/Audio/BG_Music/MSS_DoorOpen.MSS_DoorOpen" (Transformation|GetActorLocation) "0, 0, 0" 1.0 1.0 0.0 0 0 0 0)
  (bind (_direction _door3 _door3_cihuy) (Timeline|Door%203 Play)
    (:Update
      (Transformation|SetRelativeLocation (Variables|Default|GetDoor3) _door3 false false)
      (Transformation|SetRelativeLocation (Variables|Default|GetDoor3_a) _door3_cihuy false false))))

(event OnComponentEndOverlap(Box)
  (params (OverlappedComponent :type Primitive%20Component%20Object%20Reference) (OtherActor :type Actor%20Object%20Reference) (OtherComp :type Primitive%20Component%20Object%20Reference) (OtherBodyIndex :type Integer))
  (bind _asbp_macky (Utilities|Casting|CastToBP_Macky OtherActor))
  (Variables|Default|SetBP_Macky _asbp_macky)
  (Audio|PlaySoundatLocation "/Game/My_MAP/MK_Character/Audio/BG_Music/MSS_DoorOpen.MSS_DoorOpen" (Transformation|GetActorLocation) "0, 0, 0" 1.0 1.0 0.0 0 0 0 0)
  (bind (_direction _door3 _door3_cihuy) (Timeline|Door%203 Reverse)
    (:Update
      (Transformation|SetRelativeLocation (Variables|Default|GetDoor3) _door3 false false)
      (Transformation|SetRelativeLocation (Variables|Default|GetDoor3_a) _door3_cihuy false false))))

(fn ConstructionScript)