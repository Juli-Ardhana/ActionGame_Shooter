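; BP_DoorSlide2 is a sliding door that opens once enough items have been destroyed.
; Each Destroyit event increments CurrentItemDestroy, and when it reaches MaxItemDestroy a DoOnce fires DoorOpenedZ.
; DoorOpenedZ plays the Door_2 timeline, whose vector track drives the relative location of the DoorSlide2 component without sweep.
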(event Custom|Destroy%20it
  (Math|Integer|IncrementInt (Variables|Default|GetCurrentItemDestroy)
    (:%20%20
      (if (>= (Variables|Default|GetCurrentItemDestroy) (Variables|Default|GetmaxItemDestroy))
        (Utilities|FlowControl|DoOnce false
          (:Completed
            (CallFunction|DoorOpenedZ)))))))

(event Custom|Door%20Opened%20Z
  (bind _newtrack_0 (Timeline|Door_2 Play)
    (:Update
      (Transformation|SetRelativeLocation (Variables|Default|GetDoorSlide2) _newtrack_0 false false))))

(fn ConstructionScript)